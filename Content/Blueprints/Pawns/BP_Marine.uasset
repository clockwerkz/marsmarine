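; BP_Marine is a player pawn with world-axis movement and independent aiming, in the style of a twin-stick shooter.
; MoveForward and MoveRight feed movement input along world X and Y.
; Each Tick, UpdatePlayerAim turns mouse velocity above a deadzone into a yaw and smoothly interpolates the control rotation toward it.
; A thumbstick aiming branch with its own deadzone exists but is disconnected, so only mouse aim runs.
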(event Collision|EventActorBeginOverlap
  (params (OtherActor :type Actor%20Object%20Reference)))

(event EventTick
  (params (DeltaSeconds :type Float%20%28single-precision%29))
  (CallFunction|UpdatePlayerAim))

(event Input|AxisEvents|InputAxisMoveForward
  (params (AxisValue :type Float%20%28single-precision%29))
  (Pawn|Input|AddMovementInput "1.000000, 0, 0" AxisValue false))

(event Input|AxisEvents|InputAxisMoveRight
  (params (AxisValue :type Float%20%28single-precision%29))
  (Pawn|Input|AddMovementInput "0,1.000000,0.000000" AxisValue false))

(fn ConstructionScript)

(fn UpdatePlayerAim
  (bind _returnvalue (CallFunction|GetMouseVelocity))
  (bind _returnvalue_2 (Game|GetPlayerController 0))
  (if (CallFunction|IsMouseAboveDeadzone)
    (Pawn|SetControlRotation _returnvalue_2 (Math|Interpolation|RInterpTo (Pawn|GetControlRotation _returnvalue_2 :!class /Script/Engine.Controller) (Math|Rotator|MakeRotator 0.0 0.0 (Class|KismetMathLibrary|DegAtan2 (.x _returnvalue) (.y _returnvalue))) (Utilities|Time|GetWorldDeltaSeconds) (Variables|Default|GetMouseSmoothStrength)))))

(fn IsThumbstickAboveDeadzone
  (return (> (Math|Vector2D|Vector2DLength (Math|Vector2D|MakeVector2D (Input|AxisValues|GetThumbStick_AimUp) (Input|AxisValues|GetThumbStick_AimRight))) (Variables|Default|GetThumbstickDeadzone))))

(fn GetMouseVelocity
  (bind _returnvalue (Game|GetPlayerController 0))
  (bind (_deltax _deltay) (Class|PlayerController|GetInputMouseDelta _returnvalue))
  (return (Math|Conversions|ToVector2D(Vector) (/ (Math|Vector2D|MakeVector2D _deltax _deltay) (Utilities|Time|GetWorldDeltaSeconds)))))

(fn IsMouseAboveDeadzone
  (return (> (Math|Vector2D|Vector2DLength (CallFunction|GetMouseVelocity)) (Variables|Default|GetMouseDeadzone))))